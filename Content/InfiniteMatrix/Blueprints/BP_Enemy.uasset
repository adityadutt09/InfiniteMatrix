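; BP_Enemy is a spinning enemy actor that awards the player 20 points when touched.
; On overlap with BP_Player, EnemyCollision destroys the enemy, adds to the player's Score and refreshes the HUD.
; Tick rotates the actor and destroys it if EnemyLifeSpan is at or below zero.
; The lifespan decrement sits inside that same check, so a positive value never counts down here.
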(event OnComponentBeginOverlap(EnemyCollision)
  (params (OverlappedComponent :type Primitive%20Component%20Object%20Reference) (OtherActor :type Actor%20Object%20Reference) (OtherComp :type Primitive%20Component%20Object%20Reference) (OtherBodyIndex :type Integer) (bFromSweep :type Boolean) (SweepResult :type Hit%20Result%20Structure%20%28by%20ref%29))
  ;[1 1 1] Enemy Collision with Player
  (bind _asbp_player (Utilities|Casting|CastToBP_Player OtherActor))
  (Actor|DestroyActor)
  (Variables|/Game/InfiniteMatrix/Blueprints/BP_Player.BP_Player_C|SetScore _asbp_player (+ (Variables|/Game/InfiniteMatrix/Blueprints/BP_Player.BP_Player_C|GetScore _asbp_player) 20))
  (Default|UpdateScore (Variables|/Game/InfiniteMatrix/Blueprints/BP_Player.BP_Player_C|GetBP_HUD _asbp_player)))

(event EventBeginPlay
  (Actor|GetAllActorsOfClass "/Game/InfiniteMatrix/Blueprints/BP_Player.BP_Player_C"))

(event Collision|EventActorBeginOverlap
  (params (OtherActor :type Actor%20Object%20Reference)))

(event EventTick
  (params (DeltaSeconds :type Float%20%28single-precision%29))
  ;[1 1 1] Destroying after Lifespan
  (Transformation|AddActorLocalRotation "2.000000, 0, 0" false false)
  (if (<= (Variables|Default|GetEnemyLifeSpan) 0.0)
    (Variables|Default|SetEnemyLifeSpan (- (Variables|Default|GetEnemyLifeSpan) DeltaSeconds))
    (Actor|DestroyActor)))

(fn ConstructionScript)