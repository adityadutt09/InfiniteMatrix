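; BP_Tunnel is an endless tunnel segment with a rotating wall that the player must avoid hitting.
; Passing its trigger has TunnelSpawner add another tunnel, destroys this one and awards score.
; Wall hits cost score and health, driving the HUD and a low-health post-process blend, with pause and restart on death.
; Helper functions, not called here, randomize the wall's hole mesh and roll and spawn offset health packs and enemies.
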(event OnComponentBeginOverlap(TriggerZone)
  (params (OverlappedComponent :type Primitive%20Component%20Object%20Reference) (OtherActor :type Actor%20Object%20Reference) (OtherComp :type Primitive%20Component%20Object%20Reference) (OtherBodyIndex :type Integer) (bFromSweep :type Boolean) (SweepResult :type Hit%20Result%20Structure%20%28by%20ref%29))
  ;[1 1 1] Spawn Tunnels
  (bind _asbp_player (Utilities|Casting|CastToBP_Player OtherActor))
  (Default|SpawnTunnelatSpawnPoint (Variables|Default|GetTunnelSpawner))
  (Actor|DestroyActor)
  (Variables|/Game/InfiniteMatrix/Blueprints/BP_Player.BP_Player_C|SetScore _asbp_player (+ (Variables|/Game/InfiniteMatrix/Blueprints/BP_Player.BP_Player_C|GetScore _asbp_player) 15)))

(event OnComponentEndOverlap(TriggerZone)
  (params (OverlappedComponent :type Primitive%20Component%20Object%20Reference) (OtherActor :type Actor%20Object%20Reference) (OtherComp :type Primitive%20Component%20Object%20Reference) (OtherBodyIndex :type Integer))
  ;[1 1 1] Display Score After Passing Trigger Zone
  (bind _asbp_player (Utilities|Casting|CastToBP_Player OtherActor))
  (Default|UpdateScore (Variables|/Game/InfiniteMatrix/Blueprints/BP_Player.BP_Player_C|GetBP_HUD _asbp_player)))

(event OnComponentBeginOverlap(WallMesh)
  (params (OverlappedComponent :type Primitive%20Component%20Object%20Reference) (OtherActor :type Actor%20Object%20Reference) (OtherComp :type Primitive%20Component%20Object%20Reference) (OtherBodyIndex :type Integer) (bFromSweep :type Boolean) (SweepResult :type Hit%20Result%20Structure%20%28by%20ref%29))
  ;[1 1 1] Check for Collision with Wall
  (bind _asbp_player (Utilities|Casting|CastToBP_Player OtherActor))
  (CallFunction|ProcessHit _asbp_player)
  (Variables|/Game/InfiniteMatrix/Blueprints/BP_Player.BP_Player_C|SetScore _asbp_player (- (Variables|/Game/InfiniteMatrix/Blueprints/BP_Player.BP_Player_C|GetScore _asbp_player) 15))
  (if (Variables|/Game/InfiniteMatrix/Blueprints/BP_Player.BP_Player_C|GetIsDead _asbp_player)
    (Variables|/Game/InfiniteMatrix/Blueprints/BP_Player.BP_Player_C|SetScore _asbp_player 0)
    (Components|DestroyComponent (Variables|Default|GetWallMesh))))

(event EventBeginPlay
  (Game|SetGamePaused false))

(event EventTick
  (params (DeltaSeconds :type Float%20%28single-precision%29))
  ;[1 1 1] Spawn Wall Meshes
  (Transformation|AddLocalRotation (Variables|Default|GetWallMesh) (Math|Rotator|MakeRotator (* DeltaSeconds (Variables|Default|GetRotateSpeed)) 0.0 0.0) false false))

(fn ConstructionScript)

(fn RandomizeWall
  (Components|StaticMesh|SetStaticMesh (Variables|Default|GetWallMesh) (Utilities|Select :Index (Math|Random|RandomIntegerinRange 0 3) :Option%200 "/Game/InfiniteMatrix/Meshes/SM_Hole_01.SM_Hole_01" :Option%201 "/Game/InfiniteMatrix/Meshes/SM_Hole_02.SM_Hole_02" :Option%202 "/Game/InfiniteMatrix/Meshes/SM_Hole_03.SM_Hole_03" :Option%203 "/Game/InfiniteMatrix/Meshes/SM_Hole_04.SM_Hole_04"))
  (Transformation|AddLocalRotation (Variables|Default|GetWallMesh) (Math|Rotator|MakeRotator (Math|Random|RandomFloatinRange 0.0 3.6e+02) 0.0 0.0) false false))

(fn ProcessHit
  (params (BP_Player :type BP%20Player%20Object%20Reference))
  ;[1 1 1] Update Player Health and Score
  (bind _output_get (LocalVariables|SetPlayer BP_Player))
  (bind _output_get_2 (Variables|/Game/InfiniteMatrix/Blueprints/BP_Player.BP_Player_C|SetHealth _output_get (- (Variables|/Game/InfiniteMatrix/Blueprints/BP_Player.BP_Player_C|GetHealth (LocalVariables|GetPlayer)) 1e+01)))
  (Default|UpdateHealthBar (Variables|/Game/InfiniteMatrix/Blueprints/BP_Player.BP_Player_C|GetBP_HUD (LocalVariables|GetPlayer)) _output_get_2)
  (Variables|/Script/Engine.PostProcessComponent|SetBlendWeight (Variables|/Game/InfiniteMatrix/Blueprints/BP_Player.BP_Player_C|GetPostProcess (LocalVariables|GetPlayer)) (Math|Float|MapRangeClamped _output_get_2 5e+01 1e+01 0.0 1.0))
  (if (<= (Variables|/Game/InfiniteMatrix/Blueprints/BP_Player.BP_Player_C|GetHealth (LocalVariables|GetPlayer)) 0.0)
    (Variables|/Game/InfiniteMatrix/Blueprints/BP_Player.BP_Player_C|SetIsDead (LocalVariables|GetPlayer) true)
    (Default|DisplayRestart (LocalVariables|GetPlayer))
    (Game|SetGamePaused true)
    (bind _output_get_3 (Variables|/Game/InfiniteMatrix/Blueprints/BP_Player.BP_Player_C|SetHealth (LocalVariables|GetPlayer) 1e+02))
    (Default|UpdateHealthBar (Variables|/Game/InfiniteMatrix/Blueprints/BP_Player.BP_Player_C|GetBP_HUD (LocalVariables|GetPlayer)) _output_get_3)
    (Variables|/Script/Engine.PostProcessComponent|SetBlendWeight (Variables|/Game/InfiniteMatrix/Blueprints/BP_Player.BP_Player_C|GetPostProcess (LocalVariables|GetPlayer)) 0.0)
    (Variables|/Game/InfiniteMatrix/Blueprints/BP_Player.BP_Player_C|SetScore (LocalVariables|GetPlayer) 0)))

(fn RandomizeHealthPack
  (params (SpawnLocation :type Vector))
  (Game|SpawnActorfromClass "/Game/InfiniteMatrix/Blueprints/BP_HealthPack.BP_HealthPack_C" (Math|Transform|MakeTransform (Math|Vector|MakeVector (+ (.x SpawnLocation) 1e+03) (+ (.y SpawnLocation) (Math|Random|RandomFloatinRange -4e+02 4e+02)) (+ (.z SpawnLocation) (Math|Random|RandomFloatinRange -2e+02 2e+02))) "0, 0, 0" "1,1,1") "Undefined" 0 0))

(fn RandomizeEnemy
  (params (Spawn%20Location :type Vector))
  (Game|SpawnActorfromClass "/Game/InfiniteMatrix/Blueprints/BP_Enemy.BP_Enemy_C" (Math|Transform|MakeTransform (Math|Vector|MakeVector (+ (.x Spawn%20Location) 1.25e+03) (+ (.y Spawn%20Location) (Math|Random|RandomFloatinRange -4e+02 4e+02)) (+ (.z Spawn%20Location) (Math|Random|RandomFloatinRange -2e+02 2e+02))) "0, 0, 0" "1,1,1") "Undefined" 0 0))