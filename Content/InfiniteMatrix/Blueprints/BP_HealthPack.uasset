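; BP_HealthPack is a spinning health pickup that restores a fixed amount of the player's Health, capped at 100.
; Overlapping HealthMesh with a BP_Player updates that Health, refreshes the health bar through the player's BPHUD, and destroys the pack.
; Tick rotates the actor by a fixed step per frame and destroys it if HealthLifeSpan is at or below zero.
; HealthLifeSpan only decrements inside that branch, so a positive value never counts down.
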(event OnComponentBeginOverlap(HealthMesh)
  (params (OverlappedComponent :type Primitive%20Component%20Object%20Reference) (OtherActor :type Actor%20Object%20Reference) (OtherComp :type Primitive%20Component%20Object%20Reference) (OtherBodyIndex :type Integer) (bFromSweep :type Boolean) (SweepResult :type Hit%20Result%20Structure%20%28by%20ref%29))
  ;[1 1 1] Collision with Player Update Health
  (bind _asbp_player (Utilities|Casting|CastToBP_Player OtherActor))
  (if (> (+ (Variables|/Game/InfiniteMatrix/Blueprints/BP_Player.BP_Player_C|GetHealth _asbp_player) 2e+01) 1e+02)
    (bind _output_get (Variables|/Game/InfiniteMatrix/Blueprints/BP_Player.BP_Player_C|SetHealth _asbp_player 1e+02))
    (Default|UpdateHealthBar (Variables|/Game/InfiniteMatrix/Blueprints/BP_Player.BP_Player_C|GetBP_HUD _asbp_player) _output_get)
    (Actor|DestroyActor)
    (else
      (bind _output_get_2 (Variables|/Game/InfiniteMatrix/Blueprints/BP_Player.BP_Player_C|SetHealth _asbp_player (+ (Variables|/Game/InfiniteMatrix/Blueprints/BP_Player.BP_Player_C|GetHealth _asbp_player) 2e+01)))
      (Default|UpdateHealthBar (Variables|/Game/InfiniteMatrix/Blueprints/BP_Player.BP_Player_C|GetBP_HUD _asbp_player) _output_get_2)
      (Actor|DestroyActor))))

(event EventBeginPlay)

(event Collision|EventActorBeginOverlap
  (params (OtherActor :type Actor%20Object%20Reference)))

(event EventTick
  (params (DeltaSeconds :type Float%20%28single-precision%29))
  ;[1 1 1] Destroying after Lifespan
  (Transformation|AddActorLocalRotation "2.000000, 0, 0" false false)
  (if (<= (Variables|Default|GetHealthLifeSpan) 0.0)
    (Variables|Default|SetHealthLifeSpan (- (Variables|Default|GetHealthLifeSpan) DeltaSeconds))
    (Actor|DestroyActor)))

(fn ConstructionScript)